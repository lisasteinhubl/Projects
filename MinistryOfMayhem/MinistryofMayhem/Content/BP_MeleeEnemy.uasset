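; BP_MeleeEnemy is a melee enemy Blueprint that drives its overhead-style health bar widget; no combat or movement logic appears here.
; Each Tick calls GetHealth, then casts the widget to BP_EnemyHealthBar and sets its progress bar from Health as a fraction of 100.
; It also rotates the Scene component on yaw only to face the player character, billboard-style, whenever that cast succeeds.
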(event `self.ReceiveTick`
  (params (DeltaSeconds :type "Float (single-precision)"))
  (bind _scene (`self.Scene`))
  (`|ExecutionSequence`
    (:`then_0`
      (`self.GetHealth` self))
    (:`then_1`
      (bind _asbp_enemy_health_bar (cast `/Game/BP_EnemyHealthBar` (`WidgetComponent.GetUserWidgetObject` (`self.HealthBarWidget`))))
      (`ProgressBar.SetPercent` (`/Game/BP_EnemyHealthBar.ProgressBar_95` _asbp_enemy_health_bar) (/ (`self.Health`) 100.0))
      (`SceneComponent.K2_SetWorldRotation` _scene (`KismetMathLibrary.MakeRotator` 0.0 0.0 (.yaw (`KismetMathLibrary.FindLookAtRotation` (`SceneComponent.K2_GetComponentLocation` _scene) (`self.K2_GetActorLocation` (`GameplayStatics.GetPlayerCharacter` 0))))) false false))))

(fn `UserConstructionScript`)